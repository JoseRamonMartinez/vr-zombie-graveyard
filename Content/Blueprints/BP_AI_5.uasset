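; BP_AI_5 is a zombie AI that plays its sounds and chases the player pawn while the GVR_Pawn Menu flag is true.
; Tick feeds movement input toward the player, scaled by AISpeed and delta time, and yaws the capsule to face them.
; Within a small tolerance it sets Wait, plays idle, then restores the animation Blueprint after a random delay.
; A looping timer also randomizes WhereToGo, which this graph never reads.
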(event Custom|RandoLocation
  ;[1 1 1] To move a zombie to a specific position
  (Variables|Default|SetWhereToGo (Math|Random|RandomIntegerinRange 0 3)))

(event EventBeginPlay
  ;[1 1 1] To move a zombie to a specific position
  (Utilities|Time|SetTimerbyEvent (delegate Custom|RandoLocation) 2.0 true)
  (Audio|Components|Audio|Stop (Variables|Default|Getzombie)))

(event Collision|EventActorBeginOverlap
  (params (OtherActor :type Actor%20Object%20Reference)))

(event EventTick
  (params (DeltaSeconds :type Float%20%28single-precision%29))
  (bind _returnvalue (Game|Player|GetPlayerPawn 0))
  (bind _capsulecomponent (Variables|Collision|GetCapsuleComponent))
  (bind _returnvalue_2 (Transformation|GetActorLocation _returnvalue))
  (bind _returnvalue_3 (Transformation|GetWorldLocation _capsulecomponent))
  ;[1 1 1] If the pawn is not in the menu
  (bind _asgvr_pawn (Utilities|Casting|CastToGVR_Pawn (Game|Player|GetPlayerPawn 0)))
  (if (Variables|/Game/Blueprints/GVR_Pawn.GVR_Pawn_C|Getmenu _asgvr_pawn)
    ;[1 1 1] Is the zombie is not playing sounds, starts the zombie sounds
    (if (Audio|Components|Audio|IsPlaying (Variables|Default|Getzombie))
      _
      (else
        (Audio|Components|Audio|Play (Variables|Default|Getzombie) 0.0)))
    ;[1 1 1] Move the zombie and rotate to pawn position
    (Class|PawnMovementComponent|AddInputVector (Variables|Character|GetCharacterMovement) (* (* (Math|Vector|Normalize (- _returnvalue_2 _returnvalue_3)) DeltaSeconds) (Variables|Default|GetAISpeed)) false)
    (Transformation|SetRelativeRotation (Variables|Collision|GetCapsuleComponent) (Math|Rotator|MakeRotator 0.0 0.0 (.Yaw (Math|Rotator|BreakRotator (Math|Rotator|FindLookatRotation (Transformation|GetWorldLocation (Variables|Collision|GetCapsuleComponent)) (Transformation|GetActorLocation (Game|Player|GetPlayerPawn 0)))))) false false)
    ;[1 1 1] If the zombie is near the pawn, it stop the animation, else, it start the animation
    (if (Math|Vector|Equal(Vector) _returnvalue_2 _returnvalue_3 2e+01)
      (Variables|Default|SetWait true)
      (Components|Animation|PlayAnimation (Variables|Character|GetMesh) "/Game/Blueprints/Assets/characteres/Animations/idle_Root_Idle.idle_Root_Idle" true)
      (Utilities|FlowControl|Delay (Math|Random|RandomFloatinRange 2.0 6.0))
      (Variables|Default|SetWhereToGo (Math|Random|RandomIntegerinRange 0 3))
      (Components|Animation|SetAnimationMode (Variables|Character|GetMesh) "AnimationBlueprint")
      (Variables|Default|SetWait false))))

(fn ConstructionScript)