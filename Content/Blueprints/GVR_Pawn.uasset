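; VR player pawn for a level where the player walks to an exit while avoiding BP_AI enemies.
; Before play starts, gazing at TraceInteractiveCube fills a ring until it activates, or a touch does so immediately, setting Menu to true.
; Tick then moves the pawn along the camera's heading with camera shake whenever the player looks down steeply.
; Nearing a hard-coded exit wins and hitting an enemy loses, both showing messages, playing sound and loading EntryLevel after a delay.
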(event EventBeginPlay
  ;[1 1 1] Set the camera at the eye level and stop the lose and win sounds
  (Class|HeadMountedDisplayFunctionLibrary|SetTrackingOrigin "Eye")
  (Transformation|SetRelativeLocation (Variables|Default|GetVRCameraRoot) (Variables|Default|GetCamera%20Height) false false)
  (Audio|Components|Audio|Stop (Variables|Default|Getwinsound))
  (Audio|Components|Audio|Stop (Variables|Default|Getlosesound)))

(event Collision|EventActorBeginOverlap
  (params (OtherActor :type Actor%20Object%20Reference)))

(event Collision|EventHit
  (params (MyComp :type Primitive%20Component%20Object%20Reference) (Other :type Actor%20Object%20Reference) (OtherComp :type Primitive%20Component%20Object%20Reference) (bSelfMoved :type Boolean) (HitLocation :type Vector :default "0, 0, 0") (HitNormal :type Vector :default "0, 0, 0") (NormalImpulse :type Vector :default "0, 0, 0") (Hit :type Hit%20Result%20Structure%20%28by%20ref%29))
  (bind _returnvalue (Utilities|GetDisplayName Other))
  ;[1 1 1] If a zombien hit the pawn
  (if (Math|Boolean|ORBoolean (Utilities|Enum|Equal(Enum) _returnvalue "BP_AI") (Utilities|Enum|Equal(Enum) _returnvalue "BP_AI_2") (Utilities|Enum|Equal(Enum) _returnvalue "BP_AI_3") (Utilities|Enum|Equal(Enum) _returnvalue "BP_AI_4") (Utilities|Enum|Equal(Enum) _returnvalue "BP_AI_5"))
    ;[1 1 1] Finish level Logic
    (Rendering|SetVisibility (Variables|Default|Getlose) true false)
    (Audio|Components|Audio|Stop (Variables|Default|Getfondo))
    (Audio|Components|Audio|Play (Variables|Default|Getlosesound) 0.0)
    (Rendering|SetVisibility (Variables|Default|Getredirigir) true false)
    (Rendering|SetVisibility (Variables|Default|Getredirigir2) true false)
    (Collision|SetCollisionEnabled (Variables|Default|GetCapsule) "NoCollision")
    (Utilities|FlowControl|Delay 6.0)
    (Game|OpenLevel(byName) "EntryLevel")))

(event EventTick
  (params (DeltaSeconds :type Float%20%28single-precision%29))
  (bind _vrcamera (Variables|Default|GetVRCamera))
  (bind _plane (Variables|Default|GetPlane))
  (bind _returnvalue (Math|Vector|GetForwardVector _vrcamera))
  (bind (_x _y) (Math|Vector|BreakVector _returnvalue))
  (if (Math|Vector|Equal(Vector) (Transformation|GetWorldLocation (Variables|Default|GetVRCamera)) "1280.000000,176.298004,239.087006" 7e+01)
    ;[1 1 1] Finish level Logic
    (Rendering|SetVisibility (Variables|Default|Getwin) true false)
    (Audio|Components|Audio|Stop (Variables|Default|Getfondo))
    (Audio|Components|Audio|Play (Variables|Default|Getwinsound) 0.0)
    (Rendering|SetVisibility (Variables|Default|Getredirigir) true false)
    (Rendering|SetVisibility (Variables|Default|Getredirigir2) true false)
    (Collision|SetCollisionEnabled (Variables|Default|GetCapsule) "NoCollision")
    (Utilities|FlowControl|Delay 6.0)
    (Game|OpenLevel(byName) "EntryLevel")
    (else
      ;[1 1 1] If the menu is active or not
      (if (Variables|Default|Getmenu)
        ;[1 1 1] Movement interacction
        (if (< (.Pitch (Math|Rotator|BreakRotator (Transformation|GetWorldRotation (Variables|Default|GetVRCamera)))) -38.0)
          (Pawn|Input|AddMovementInput self (Math|Vector|MakeVector _x _y 0.0) 1.0 false)
          (Camera|PlayWorldCameraShake "/Game/Blueprints/CameraShake.CameraShake_C" (Transformation|GetWorldLocation (Variables|Default|GetVRCamera)) 0.0 5e+02))
        (elif (Utilities|Name|Equal(Name) "TraceInteractiveCube" (Utilities|String|StringToName (Utilities|GetDisplayName (.HitActor (Collision|BreakHitResult (Variables|/Game/Blueprints/Components/TraceInteraction-Component.TraceInteraction-Component_C|GetInHit (Variables|Default|GetTraceInteraction-Component)))))))
          (Rendering|SetVisibility (Variables|Default|GetPlane) true false)
          (if (Math|Float|NearlyEqual(Float) (Variables|Default|Getcount) 1.0 0.0001)
            (Default|ActiveDown (Variables|Default|GetTraceInteraction-Component) self)
            (Rendering|Material|CreateDynamicMaterialInstance (Variables|Default|GetPlane) 0 "/Engine/BufferVisualization/AmbientOcclusion.AmbientOcclusion" :!class /Script/Engine.PrimitiveComponent)
            (Variables|Default|Setmenu true)
            (else
              (Rendering|Material|CreateDynamicMaterialInstance _plane 0 "/Game/Blueprints/Materials/UIRing.UIRing" :!class /Script/Engine.PrimitiveComponent)
              (Rendering|Material|SetScalarParameterValueonMaterials _plane "PercentComplete" (+ (Variables|Default|Getcount) 0.005))
              (Variables|Default|Setcount (+ (Variables|Default|Getcount) 0.005))))
          (else
            (Rendering|Material|CreateDynamicMaterialInstance (Variables|Default|GetPlane) 0 "/Engine/BufferVisualization/AmbientOcclusion.AmbientOcclusion" :!class /Script/Engine.PrimitiveComponent)
            (Variables|Default|Setcount 0.0)))))))

(event Input|TouchEvents|InputTouch
  (params (Location :type Vector) (FingerIndex :type ETouchIndex%20Enum))
  (bind _self self)
  (bind _traceinteraction_component (Variables|Default|GetTraceInteraction-Component))
  (:Pressed
    (Default|ActiveDown _traceinteraction_component _self)
    (Variables|Default|Setmenu true))
  (:Released
    (Default|ActiveUp _traceinteraction_component _self)))

(fn ConstructionScript)